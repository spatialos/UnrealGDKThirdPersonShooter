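; BP_StressCube is a physics cube that keeps kicking itself into motion, apparently for stress testing.
; On BeginPlay it starts a looping one-second timer that applies a fixed upward impulse to its Box.
; Impulses are applied only with authority, so the server drives the motion.
; A random-direction, random-strength Twitch variant exists, but its randomized timer is disconnected, leaving it unused.
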(event Custom|StartTwitchTimer
  (Utilities|Time|SetTimerbyEvent (delegate Custom|ControlledTwitch) 1.0 true))

(event Custom|DoTwitch
  (CallFunction|Twitch)
  (CallFunction|StartTwitchTimer))

(event Custom|ControlledTwitch
  (Networking|SwitchHasAuthority
    (:Authority
      (Physics|AddImpulse (Variables|Default|GetBox) "0, 0,50000.000000" "None" false))))

(event EventBeginPlay
  (CallFunction|StartTwitchTimer))

(fn ConstructionScript)

(fn Twitch
  (Networking|SwitchHasAuthority
    (:Authority
      (Physics|AddImpulse (Variables|Default|GetBox) (* (Math|Random|RandomUnitVector) (Math|Random|RandomFloatinRange 1e+04 2e+05)) "None" false))))