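; BigGymCharacter_BP is the character for the BigGym map that relays Q and E key presses to the world's DormantActorManager.
; Each key calls a Server-prefixed event, which looks up the manager and calls its QPressed or EPressed.
; The lookup searches all actors of that class and prints a red error unless exactly one exists.
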(event Custom|ServerQ
  (bind _instance (CallFunction|GetDormantActorManager))
  (Default|QPressed _instance))

(event Custom|ServerE
  (bind _instance (CallFunction|GetDormantActorManager))
  (Default|EPressed _instance))

(event Input|KeyboardEvents|Q
  (params (Key :type Key%20Structure))
  (:Pressed
    (CallFunction|ServerQ)))

(event Input|KeyboardEvents|E
  (params (Key :type Key%20Structure))
  (:Pressed
    (CallFunction|ServerE)))

(fn ConstructionScript)

(fn GetDormantActorManager
  (bind _outactors (Actor|GetAllActorsOfClass "/Game/UNR-1400/DormantActorManager.DormantActorManager_C"))
  (if (== (Utilities|Array|Length _outactors) 1)
    (return (Utilities|Array|Get(acopy) _outactors))
    (else
      (Development|PrintText (Utilities|Text|FormatText "Need to have exactly one dormant actor manager in the world, but found {0}" (Utilities|Array|Length _outactors)) true true "(R=1.000000,G=0.000000,B=0.000000,A=1.000000)"))))