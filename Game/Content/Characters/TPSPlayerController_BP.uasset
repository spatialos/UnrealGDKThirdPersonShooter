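; Player controller for a third-person shooter that handles aim input, camera pitch limits, and the quit and respawn screens.
; BeginPlay creates both widgets and applies the pitch limits; right mouse toggles aiming on a cached TPSCharacter_BP pawn.
; ShowRespawnScreen switches to menu input and sets a waiting flag that gates both Delete's quit-menu toggle and Space's respawn.
; RequestRespawn calls RequestServerRespawn, which runs RespawnCharacter, then restores game-only input.
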(event Custom|RequestServerRespawn
  (Class|TPSPlayerController|RespawnCharacter))

(event EventBeginPlay
  (bind _self self)
  (bind _playercameramanager (Variables|Default|GetPlayerCameraManager))
  (Utilities|FlowControl|Sequence
    (:then_0
      (Input|EnableInput 0))
    (:then_1
      (bind _returnvalue (UserInterface|CreateWidget "/Game/UI/Blueprints/BP_QuitScreen.BP_QuitScreen_C" _self))
      (Variables|Default|SetQuitMenu _returnvalue)
      (CallFunction|SetQuitMenu false))
    (:then_2
      (bind _returnvalue_2 (UserInterface|CreateWidget "/Game/UI/Blueprints/BP_RespawnMenu.BP_RespawnMenu_C" _self))
      (Variables|Default|SetRespawnScreen _returnvalue_2))
    (:then_3
      (Variables|/Script/Engine.PlayerCameraManager|SetViewPitchMax _playercameramanager (Variables|Default|GetMax%20Pitch))
      (Variables|/Script/Engine.PlayerCameraManager|SetViewPitchMin _playercameramanager (Variables|Default|GetMin%20Pitch)))))

(event Input|MouseEvents|RightMouseButton
  (params (Key :type Key%20Structure))
  (:Pressed
    (bind _controlledplayer (Utilities|GetPlayer)
      (:Is%20Valid
        (Default|SetAiming _controlledplayer true))))
  (:Released
    (bind _controlledplayer_2 (Utilities|GetPlayer)
      (:Is%20Valid
        (Default|SetAiming _controlledplayer_2 false)))))

(event Input|KeyboardEvents|SpaceBar
  (params (Key :type Key%20Structure))
  (:Pressed
    (if (Variables|Default|GetWaitingForRespawn)
      (CallFunction|RequestRespawn self))))

(event Input|KeyboardEvents|Delete
  (params (Key :type Key%20Structure))
  (:Pressed
    (if (Variables|Default|GetWaitingForRespawn)
      (CallFunction|SetQuitMenu (not (Variables|Default|GetInMenu))))))

(fn ConstructionScript)

(fn SetQuitMenu
  (params (InMenu :type Boolean))
  (bind _self self)
  (bind _quitmenu (Variables|Default|GetQuitMenu))
  (bind _output_get (Variables|Default|SetInMenu InMenu))
  (Utilities|IsValid _quitmenu
    (:Is%20Valid
      (if _output_get
        (UserInterface|Viewport|AddtoViewport _quitmenu 0)
        (Input|SetInputModeGameandUI _self _quitmenu "DoNotLock" false)
        (else
          (Widget|RemovefromParent _quitmenu)
          (Input|SetInputModeGameOnly _self :!label _label))))
    (:Is%20Not%20Valid
      (goto _label)))
  (Variables|/Script/Engine.PlayerController|SetbShowMouseCursor _self (Variables|Default|GetInMenu)))

(fn ShowRespawnScreen
  (bind _self self)
  (bind _respawnscreen (Variables|Default|GetRespawnScreen))
  (if (not (Variables|Default|GetWaitingForRespawn))
    (Variables|Default|SetWaitingForRespawn true)
    (CallFunction|SetQuitMenu false)
    (UserInterface|Viewport|AddtoViewport _respawnscreen 0)
    (Default|Initialise _respawnscreen _self)
    (Input|SetInputModeGameandUI _self _respawnscreen "DoNotLock" false)
    (bind _output_get (Variables|Default|SetInMenu true))
    (Variables|/Script/Engine.PlayerController|SetbShowMouseCursor _self _output_get)))

(fn RequestRespawn
  (bind _self self)
  (if (Variables|Default|GetWaitingForRespawn)
    (CallFunction|RequestServerRespawn)
    (Variables|Default|SetWaitingForRespawn false)
    (Widget|RemovefromParent (Variables|Default|GetRespawnScreen))
    (Input|SetInputModeGameOnly _self)
    (bind _output_get (Variables|/Script/Engine.PlayerController|SetbShowMouseCursor _self false))
    (Variables|Default|SetInMenu _output_get)))