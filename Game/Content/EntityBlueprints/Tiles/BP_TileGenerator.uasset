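; BP_TileGenerator builds a seeded, square arena from tile actors attached to itself.
; GenerateTiles clears previous attachments, then walks a spiral from the centre, placing four fixed centre tiles and randomly rotated random or empty tiles beyond.
; Optional per-side flags add edge floors, walls with taller invisible collision, and corners.
; Finally, capsule traces snap attached UnselectedTeamPlayerStart_BP spawns to the ground, warning when none is found.
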(event EventBeginPlay)

(event Collision|EventActorBeginOverlap
  (params (OtherActor :type Actor%20Object%20Reference)))

(event EventTick
  (params (DeltaSeconds :type Float%20%28single-precision%29)))

(fn ConstructionScript)

(fn GenerateTiles
  (|CalculateCenteringOffset)
  (|Initrandomseed)
  (GenerationOptions|DeleteAllChildren)
  (bind _output_get (LocalVariables|SetTileCount (|Calculate#Tiles)))
  (for _index (range 0 (- _output_get 1))
    (|GenerateTiles _index))
  (for _index_2 (range 0 (|(({22869766-434A-BE69-EEC6-39AE1EA370BB}*2)-2)))
    (|GenerateWallsandEdges _index_2))
  (|Makecorners)
  (Utility|SnapSpawnstoGround))

(fn PlaceTileatCoordinate
  (params (Coordinate :type Int%20Vector%20Structure) (Tile :type BP%20Tile%20Base%20Class%20Reference) (Rotation :type Float%20%28single-precision%29))
  (LocalVariables|SetTileOffset (/ (Variables|InternalSettingsandVars|GetTileSizeInMeters) 2.0))
  (bind _returnvalue (Game|SpawnActorfromClass Tile (Math|Transform|MakeTransform (* (+ (Math|Vector|MakeVector (|(((tileCoordX-1)*{51612C78-44D7-435B-D762-52A4696B2B77})+{1B35EFCC-4E8A-3897-E568-569F569B32C7}) (Math|Conversions|ToFloat(Integer) (.x Coordinate))) (|(((tileCoordY-1)*{51612C78-44D7-435B-D762-52A4696B2B77})+{1B35EFCC-4E8A-3897-E568-569F569B32C7}) (Math|Conversions|ToFloat(Integer) (.y Coordinate))) 0.0) (Variables|Default|GetCentering%20Offset)) 100) (Math|Rotator|MakeRotator 0.0 0.0 Rotation) "1,1,1") "Undefined" 0 0))
  (Transformation|AttachActorToActor _returnvalue self "None" "KeepRelative" "KeepRelative" "KeepRelative" true))

(fn GetRandomTile
  (bind _tiles (Variables|InternalReferenceVars|GetTiles))
  (return (Utilities|Array|Get(acopy) _tiles (Class|KismetMathLibrary|RandomIntegerfromStream (Utilities|Array|Length _tiles) (Variables|InternalSettingsAndVars|GetRandomStream)))))

(fn MakePlane
  (params (Spawn%20Transform%20Location :type Vector) (Spawn%20Transform%20Rotation :type Rotator) (Spawn%20Transform%20Scale :type Vector) (Material :type Material%20Interface%20Object%20Reference) (Collision%20only :type Boolean))
  (bind _returnvalue (Game|SpawnActorfromClass "/Script/Engine.StaticMeshActor" (Math|Transform|MakeTransform Spawn%20Transform%20Location Spawn%20Transform%20Rotation Spawn%20Transform%20Scale) "Undefined" 0 0))
  (Transformation|AttachActorToActor _returnvalue self "None" "KeepRelative" "KeepRelative" "KeepRelative" true)
  (Components|StaticMesh|SetStaticMesh (Variables|/Script/Engine.StaticMeshActor|GetStaticMeshComponent _returnvalue) "/Engine/BasicShapes/Plane.Plane")
  (Rendering|Material|SetMaterial (Variables|/Script/Engine.StaticMeshActor|GetStaticMeshComponent _returnvalue) 0 Material)
  (Rendering|SetVisibility (Variables|/Script/Engine.StaticMeshActor|GetStaticMeshComponent _returnvalue) (not Collision%20only) false)
  (return))

(fn MakeOutsideWall
  (params (WallPlaneLocation :type Vector) (SpawnTransformRotation :type Rotator) (Width :type Float%20%28single-precision%29))
  (Utility|MakeCube WallPlaneLocation SpawnTransformRotation (Math|Vector|MakeVector Width 4.0 4.0) (Variables|InternalReferenceVars|GetWallMaterial) false)
  (Utility|MakeCube (+ WallPlaneLocation "0,0.000000,600.000000") SpawnTransformRotation (Math|Vector|MakeVector Width 4.0 8.0) 0 true)
  (return))

(fn DeleteAllChildren
  (bind _children (CallFunction|GetAllAttachedActors self))
  (for _array_element _children
    (Actor|DestroyActor _array_element)))

(fn SnapSpawnstoGround
  (bind _children (CallFunction|GetAllAttachedActors self))
  (for _array_element _children
    (bind _asunselected_team_player_start_bp (Utilities|Casting|CastToUnselectedTeamPlayerStart_BP _array_element))
    (bind (_outhit _returnvalue) (Collision|CapsuleTraceByChannel (Transformation|GetActorLocation _asunselected_team_player_start_bp) (+ (Transformation|GetActorLocation _asunselected_team_player_start_bp) (Math|Vector|MakeVector 0.0 0.0 (* (Variables|InternalSettingsandVars|GetDistanceToCheckBelowSpawnForSnap) -1.0))) (Variables|InternalSettingsandVars|GetPlayerCapsuleRadius) (Variables|InternalSettingsandVars|GetPlayerCapsuleHalfHeight) "TraceTypeQuery1" true 0 "None" false "(R=1.000000,G=0.000000,B=0.000000,A=1.000000)" "(R=0.000000,G=1.000000,B=0.000000,A=1.000000)" 2e+01))
    (if _returnvalue
      (Transformation|SetActorLocation _asunselected_team_player_start_bp (.location _outhit) false true)
      (else
        (Development|PrintString (Utilities|String|Append "Warning: Spawn found with no ground below! Spawn = " (Utilities|GetDisplayName _asunselected_team_player_start_bp)) true true "(R=1.000000,G=0.000000,B=0.000000,A=1.000000)")))))

(fn MakeCube
  (params (Spawn%20Transform%20Location :type Vector) (Spawn%20Transform%20Rotation :type Rotator) (Spawn%20Transform%20Scale :type Vector) (Material :type Material%20Interface%20Object%20Reference) (Collision%20only :type Boolean))
  (bind _returnvalue (Game|SpawnActorfromClass "/Script/Engine.StaticMeshActor" (Math|Transform|MakeTransform Spawn%20Transform%20Location Spawn%20Transform%20Rotation Spawn%20Transform%20Scale) "Undefined" 0 0))
  (Transformation|AttachActorToActor _returnvalue self "None" "KeepRelative" "KeepRelative" "KeepRelative" true)
  (Components|StaticMesh|SetStaticMesh (Variables|/Script/Engine.StaticMeshActor|GetStaticMeshComponent _returnvalue) "/Game/Environment/Props/Meshes/SM_Cube_1m.SM_Cube_1m")
  (Rendering|Material|SetMaterial (Variables|/Script/Engine.StaticMeshActor|GetStaticMeshComponent _returnvalue) 0 Material)
  (Rendering|SetVisibility (Variables|/Script/Engine.StaticMeshActor|GetStaticMeshComponent _returnvalue) (not Collision%20only) false)
  (return))